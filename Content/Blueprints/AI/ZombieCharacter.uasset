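; Zombie enemy character that turns to face the player on spawn, tracks health and ragdolls on death.
; MinusHealth updates the AiLifeWidget and, at zero, disables capsule collision and notifies the player's FPCharacterTrace.
; Trace callbacks toggle custom-depth highlighting and the life bar for one trace type while the game is unpaused.
; ActivatePause freezes or resumes the zombie through CustomTimeDilation, following the player's pause flag.
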(event `self.ReceiveBeginPlay`
  (`self.K2_SetActorRotation` (`KismetMathLibrary.FindLookAtRotation` (`self.K2_GetActorLocation`) (`self.K2_GetActorLocation` (`GameplayStatics.GetPlayerCharacter` 0))))
  (`SceneComponent.SetVisibility` (`self.Widget`) false false))

(event `self.ReceivePossessed`
  (params (NewController :type "Controller Object Reference"))
  (bind _aszombie_animation_bp (cast `/Game/Blueprints/AI/zombieAnimationBP` (`SkeletalMeshComponent.GetAnimInstance` (`self.Mesh`))))
  (set `self.Animation` _aszombie_animation_bp))

(event `self.ReceiveTick`
  (params (DeltaSeconds :type "Float (single-precision)")))

(fn `ActivatePause`
  (bind _asfpcharacter_trace (cast `/Game/Blueprints/FPCharacterTrace` (`GameplayStatics.GetPlayerCharacter` 0)))
  (if (`/Game/Blueprints/FPCharacterTrace.isGamePaused` _asfpcharacter_trace)
    (set `self.CustomTimeDilation` 0.0)
    (else
      (set `self.CustomTimeDilation` 1.0))))

(fn `DesactivatePause`)

(fn `MinusHealth`
  (params (NewParam :type Integer))
  (bind _health (`self.Health`))
  (set `self.Health` (- (`self.Health`) NewParam))
  (bind _asai_life_widget (cast `/Game/UI/AiLifeWidget` (`WidgetComponent.GetUserWidgetObject` (`self.Widget`))))
  (`/Game/UI/AiLifeWidget.UpdateLife` _asai_life_widget (`KismetMathLibrary.Conv_IntToDouble` _health) (`KismetMathLibrary.Conv_IntToDouble` (`self.MaxHealth`)))
  (if (<= _health 0)
    (`PrimitiveComponent.SetSimulatePhysics` (`self.Mesh`) true)
    (`PrimitiveComponent.SetCollisionEnabled` (`self.CapsuleComponent`) "NoCollision")
    (set `self.IsAlive` false)
    (bind _asfpcharacter_trace (cast `/Game/Blueprints/FPCharacterTrace` (`GameplayStatics.GetPlayerCharacter` 0)))
    (`/Game/Blueprints/FPCharacterTrace.ZombieDead` _asfpcharacter_trace)))

(fn `TraceActivateDown`
  (params (hit :type "HitResult Structure (by ref)") (Instigator :type "Pawn Object Reference (by ref)") (TraceType :type "/Game/Blueprints/Interfaces/TypeTraceEnumerator Enum" :default "NewEnumerator0"))
  (returns (Return :type Boolean))
  (return false))

(fn `TraceActivateUp`
  (params (Instigator :type "Pawn Object Reference (by ref)") (hit :type "HitResult Structure (by ref)") (TraceType :type "/Game/Blueprints/Interfaces/TypeTraceEnumerator Enum" :default "NewEnumerator0"))
  (returns (Return :type Boolean))
  (return false))

(fn `TraceHitComponet`
  (params (hit :type "HitResult Structure") (component :type "PrimitiveComponent Object Reference") (TraceType :type "/Game/Blueprints/Interfaces/TypeTraceEnumerator Enum" :default "NewEnumerator0"))
  (returns (Return :type Boolean))
  (return false))

(fn `TraceHitObject`
  (params (hit :type "HitResult Structure") (TraceType :type "/Game/Blueprints/Interfaces/TypeTraceEnumerator Enum" :default "NewEnumerator0"))
  (returns (Return :type Boolean))
  (bind _asfpcharacter_trace (cast `/Game/Blueprints/FPCharacterTrace` (`GameplayStatics.GetPlayerCharacter` 0)))
  (if (and (`|EnumEquality` TraceType "NewEnumerator1") (not (`/Game/Blueprints/FPCharacterTrace.isGamePaused` _asfpcharacter_trace)))
    (`PrimitiveComponent.SetRenderCustomDepth` (`self.Mesh`) true)
    (`SceneComponent.SetVisibility` (`self.Widget`) true false))
  (return false))

(fn `TraceLeaveComponent`
  (params (hit :type "HitResult Structure") (component :type "PrimitiveComponent Object Reference") (TraceType :type "/Game/Blueprints/Interfaces/TypeTraceEnumerator Enum" :default "NewEnumerator0"))
  (returns (Return :type Boolean))
  (return false))

(fn `TraceLeaveObject`
  (params (hit :type "HitResult Structure") (TraceType :type "/Game/Blueprints/Interfaces/TypeTraceEnumerator Enum" :default "NewEnumerator0"))
  (returns (Return :type Boolean))
  (bind _asfpcharacter_trace (cast `/Game/Blueprints/FPCharacterTrace` (`GameplayStatics.GetPlayerCharacter` 0)))
  (if (and (`|EnumEquality` TraceType "NewEnumerator1") (not (`/Game/Blueprints/FPCharacterTrace.isGamePaused` _asfpcharacter_trace)))
    (`PrimitiveComponent.SetRenderCustomDepth` (`self.Mesh`) false)
    (`SceneComponent.SetVisibility` (`self.Widget`) false false))
  (return false))

(fn `TraceMove`
  (params (hit :type "HitResult Structure (by ref)") (TraceType :type "/Game/Blueprints/Interfaces/TypeTraceEnumerator Enum" :default "NewEnumerator0"))
  (returns (Return :type Boolean))
  (return false))

(fn `UserConstructionScript`)