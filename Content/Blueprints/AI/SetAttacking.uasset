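; Behavior tree task that sets a zombie's attacking animation state and times its hit on the player.
; It copies its Attacking value to the animation's IsAttacking flag, finishing immediately when false.
; When true, delays time the swing: after a wind-up it calls Hit on player 0's character if the zombie is alive, with no range check.
; It then waits out the recovery before finishing successfully, skipping that wait if the zombie died.
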(event `self.ReceiveExecuteAI`
  (params (OwnerController :type "AIController Object Reference") (ControlledPawn :type "Pawn Object Reference"))
  (bind _aszombie_character (cast `/Game/Blueprints/AI/ZombieCharacter` ControlledPawn))
  (bind _output_get (set `/Game/Blueprints/AI/zombieAnimationBP.isAttacking` (`self.attacking`) (`/Game/Blueprints/AI/ZombieCharacter.Animation` _aszombie_character)))
  (if _output_get
    (`KismetSystemLibrary.Delay` 1.0)
    (bind _asfpcharacter_trace (cast `/Game/Blueprints/FPCharacterTrace` (`GameplayStatics.GetPlayerCharacter` 0)))
    (if (`/Game/Blueprints/AI/ZombieCharacter.IsAlive` _aszombie_character)
      (`/Game/Blueprints/FPCharacterTrace.Hit` _asfpcharacter_trace)
      (`KismetSystemLibrary.Delay` 1.63)))
  (`self.FinishExecute` true))