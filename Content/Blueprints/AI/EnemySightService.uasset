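; Behavior tree service that tracks a zombie's distance to and sight of the player through blackboard keys.
; On activation it targets player character 0, clears the zombie's attacking animation flag and seeds Near with a large distance.
; Each tick updates Near and line-traces to the target, ignoring all zombies.
; PlayerDetected updates only when the trace hits a Character, so other results leave it unchanged.
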(event `self.ReceiveActivationAI`
  (params (OwnerController :type "AIController Object Reference") (ControlledPawn :type "Pawn Object Reference"))
  (`BTFunctionLibrary.SetBlackboardValueAsObject` (`self.TargetActor`) (`GameplayStatics.GetPlayerCharacter` 0))
  (bind _aszombie_character (cast `/Game/Blueprints/AI/ZombieCharacter` ControlledPawn))
  (set `/Game/Blueprints/AI/zombieAnimationBP.isAttacking` false (`/Game/Blueprints/AI/ZombieCharacter.Animation` _aszombie_character))
  (`BTFunctionLibrary.SetBlackboardValueAsFloat` (`self.near`) 10000.0))

(event `self.ReceiveTickAI`
  (params (OwnerController :type "AIController Object Reference") (ControlledPawn :type "Pawn Object Reference") (DeltaSeconds :type "Float (single-precision)"))
  (bind _returnvalue (`Actor.K2_GetActorLocation` ControlledPawn))
  (bind _returnvalue_2 (`Actor.K2_GetActorLocation` (`BTFunctionLibrary.GetBlackboardValueAsActor` (`self.TargetActor`))))
  (`|ExecutionSequence`
    (:`then_0`
      (`BTFunctionLibrary.SetBlackboardValueAsFloat` (`self.near`) (`KismetMathLibrary.VSize` (- _returnvalue_2 _returnvalue))))
    (:`then_1`
      (bind _outactors (`GameplayStatics.GetAllActorsOfClass` "/Game/Blueprints/AI/ZombieCharacter.ZombieCharacter_C"))
      (bind _outhit (`KismetSystemLibrary.LineTraceSingle` _returnvalue _returnvalue_2 "TraceTypeQuery2" false _outactors))
      (bind _ascharacter (cast `Character` (`.HitActor` (`GameplayStatics.BreakHitResult` _outhit))))
      (bind _returnvalue_3 (== _ascharacter (`GameplayStatics.GetPlayerCharacter` 0)))
      (`KismetSystemLibrary.PrintString` (`KismetStringLibrary.Conv_BoolToString` _returnvalue_3) false)
      (`BTFunctionLibrary.SetBlackboardValueAsBool` (`self.PlayerDetected`) _returnvalue_3))))