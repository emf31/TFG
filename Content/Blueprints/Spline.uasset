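; Spline actor that builds a deformed mesh path from an editable array of points at construction time.
; The construction script clears the spline and adds each Points entry as a local-space spline point.
; CreateSplineMeshFromPoints then spawns a spline mesh component per segment, using the configured mesh and forward axis, with start and end positions and tangents taken from the spline.
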(fn `CreateSplineMeshFromPoints`
  (bind _spline (`self.Spline`))
  (bind _spline_2 (`self.Spline`))
  (for _index (range (+ (- (`SplineComponent.GetNumberOfSplinePoints` _spline) 2) 1))
    (bind _returnvalue (`AddComponent|NODE_AddSplineMeshComponent-3`))
    (`StaticMeshComponent.SetStaticMesh` _returnvalue (`self.StaticMesh`))
    (`SplineMeshComponent.SetForwardAxis` _returnvalue (`self.ForwardAxis`) true)
    (`SceneComponent.K2_AttachToComponent` _returnvalue _spline "None" "KeepRelative" "KeepRelative" "KeepRelative" true)
    (bind _returnvalue_2 (+ _index 1))
    (`SplineMeshComponent.SetStartAndEnd` _returnvalue (`SplineComponent.GetLocationAtSplinePoint` _spline_2 _index "Local") (`SplineComponent.GetTangentAtSplinePoint` _spline_2 _index "Local") (`SplineComponent.GetLocationAtSplinePoint` _spline_2 _returnvalue_2 "Local") (`SplineComponent.GetTangentAtSplinePoint` _spline_2 _returnvalue_2 "Local") true)))

(fn `UserConstructionScript`
  (bind _spline (`self.Spline`))
  (`SplineComponent.ClearSplinePoints` _spline true)
  (for _array_element (`self.Points`)
    (`SplineComponent.AddSplinePoint` _spline _array_element "Local" true))
  (`self.CreateSplineMeshFromPoints`))