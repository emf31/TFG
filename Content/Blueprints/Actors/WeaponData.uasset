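; Actor that shows an in-world weapon info card with a buy button, filled from a linked weapon actor.
; On BeginPlay it writes that weapon's stats, name and price into its WeaponFicha widget, registers itself on the weapon and hides.
; Trace callbacks drive a WidgetInteraction component with custom hit results and simulated left clicks.
; The button passes the weapon to FPCharacterTrace's BuyWeapon, while ShowWidget toggles visibility and collision.
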(event `self.ReceiveBeginPlay`
  (bind _asweapon_ficha (cast `/Game/UI/WeaponFicha` (`WidgetComponent.GetUserWidgetObject` (`self.Widget`))))
  (set `self.MenuWidgetObject` _asweapon_ficha)
  (`self.FillData`)
  (set `/Game/Blueprints/Actors/Weapon/Weapon.FichaWeapon` self (`self.weaponactor`))
  (`self.showWidget` false)
  (add `Button.OnClicked` (`/Game/UI/WeaponFicha.Button_170` (`self.MenuWidgetObject`)) (delegate `Buy weapon event`)))

(event `Buy weapon event`
  (bind _asfpcharacter_trace (cast `/Game/Blueprints/FPCharacterTrace` (`GameplayStatics.GetPlayerCharacter` 0)))
  (`/Game/Blueprints/FPCharacterTrace.BuyWeapon` _asfpcharacter_trace (`self.weaponactor`)))

(fn `FillData`
  (bind _weaponactor (`self.weaponactor`))
  (bind _menuwidgetobject (`self.MenuWidgetObject`))
  (bind _misautomatic (`/Game/UI/WeaponFicha.misautomatic` _menuwidgetobject))
  (`TextBlock.SetText` (`/Game/UI/WeaponFicha.mdamage` _menuwidgetobject) (`KismetTextLibrary.Conv_IntToText` (`/Game/Blueprints/Actors/Weapon/Weapon.Damage` _weaponactor)))
  (`TextBlock.SetText` (`/Game/UI/WeaponFicha.mfiringrate` _menuwidgetobject) (`KismetTextLibrary.Conv_DoubleToText` (`/Game/Blueprints/Actors/Weapon/Weapon.RateOfFire` _weaponactor) "HalfToEven"))
  (`TextBlock.SetText` (`/Game/UI/WeaponFicha.mreload` _menuwidgetobject) (`KismetTextLibrary.Conv_DoubleToText` (`/Game/Blueprints/Actors/Weapon/Weapon.ReloadTime` _weaponactor) "HalfToEven"))
  (`TextBlock.SetText` (`/Game/UI/WeaponFicha.mrange` _menuwidgetobject) (`KismetTextLibrary.Conv_IntToText` (`/Game/Blueprints/Actors/Weapon/Weapon.Range` _weaponactor)))
  (`TextBlock.SetText` (`/Game/UI/WeaponFicha.mname` _menuwidgetobject) (`KismetTextLibrary.Conv_StringToText` (`/Game/Blueprints/Actors/Weapon/Weapon.Name` _weaponactor)))
  (switch `/Game/Blueprints/Actors/Weapon/TypeOfShoot` (`/Game/Blueprints/Actors/Weapon/Weapon.ShootType` _weaponactor)
    (:`NewEnumerator0`
      (`TextBlock.SetText` _misautomatic "Automatic"))
    (:`NewEnumerator1`
      (`TextBlock.SetText` _misautomatic "SemiAutomatic")))
  (`TextBlock.SetText` (`/Game/UI/WeaponFicha.mprice` _menuwidgetobject) (`KismetTextLibrary.Conv_StringToText` (`KismetStringLibrary.Concat_StrStr` (`KismetStringLibrary.Conv_IntToString` (`/Game/Blueprints/Actors/Weapon/Weapon.Price` _weaponactor)) "$"))))

(fn `showWidget`
  (params (visible :type Boolean))
  (`self.SetActorHiddenInGame` (not visible))
  (`self.SetActorEnableCollision` visible))

(fn `TraceActivateDown`
  (params (hit :type "HitResult Structure (by ref)") (Instigator :type "Pawn Object Reference (by ref)") (TraceType :type "/Game/Blueprints/Interfaces/TypeTraceEnumerator Enum" :default "NewEnumerator0"))
  (returns (Return :type Boolean))
  (`WidgetInteractionComponent.PressPointerKey` (`self.WidgetInteraction`) "LeftMouseButton")
  (return false))

(fn `TraceActivateUp`
  (params (Instigator :type "Pawn Object Reference (by ref)") (hit :type "HitResult Structure (by ref)") (TraceType :type "/Game/Blueprints/Interfaces/TypeTraceEnumerator Enum" :default "NewEnumerator0"))
  (returns (Return :type Boolean))
  (`WidgetInteractionComponent.ReleasePointerKey` (`self.WidgetInteraction`) "LeftMouseButton")
  (return false))

(fn `TraceHitComponet`
  (params (hit :type "HitResult Structure") (component :type "PrimitiveComponent Object Reference") (TraceType :type "/Game/Blueprints/Interfaces/TypeTraceEnumerator Enum" :default "NewEnumerator0"))
  (returns (Return :type Boolean))
  (return false))

(fn `TraceHitObject`
  (params (hit :type "HitResult Structure") (TraceType :type "/Game/Blueprints/Interfaces/TypeTraceEnumerator Enum" :default "NewEnumerator0"))
  (returns (Return :type Boolean))
  (return false))

(fn `TraceLeaveComponent`
  (params (hit :type "HitResult Structure") (component :type "PrimitiveComponent Object Reference") (TraceType :type "/Game/Blueprints/Interfaces/TypeTraceEnumerator Enum" :default "NewEnumerator0"))
  (returns (Return :type Boolean))
  (return false))

(fn `TraceLeaveObject`
  (params (hit :type "HitResult Structure") (TraceType :type "/Game/Blueprints/Interfaces/TypeTraceEnumerator Enum" :default "NewEnumerator0"))
  (returns (Return :type Boolean))
  (return false))

(fn `TraceMove`
  (params (hit :type "HitResult Structure (by ref)") (TraceType :type "/Game/Blueprints/Interfaces/TypeTraceEnumerator Enum" :default "NewEnumerator0"))
  (returns (Return :type Boolean))
  (`WidgetInteractionComponent.SetCustomHitResult` (`self.WidgetInteraction`) hit)
  (return false))

(fn `UserConstructionScript`)