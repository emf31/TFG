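; CashActor is a world actor that displays the player's cash amount through a widget component.
; Every tick it casts player character 0 to FPCharacterTrace and the component's user widget to CashWidget.
; It then writes the character's Cash value, suffixed with a dollar sign, into the widget's Cash text.
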(event `self.ReceiveTick`
  (params (DeltaSeconds :type "Float (single-precision)"))
  (bind _asfpcharacter_trace (cast `/Game/Blueprints/FPCharacterTrace` (`GameplayStatics.GetPlayerCharacter` 0)))
  (bind _ascash_widget (cast `/Game/UI/CashWidget` (`WidgetComponent.GetUserWidgetObject` (`self.Widget`))))
  (`TextBlock.SetText` (`/Game/UI/CashWidget.Cash` _ascash_widget) (`KismetTextLibrary.Conv_StringToText` (`KismetStringLibrary.Concat_StrStr` (`KismetStringLibrary.Conv_IntToString` (`/Game/Blueprints/FPCharacterTrace.cash` _asfpcharacter_trace)) "$"))))

(fn `UserConstructionScript`)