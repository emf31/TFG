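; World actor with a widget Start button that begins a wave.
; On BeginPlay it binds the StartRoundWIdget button, whose click calls CallStartWave on player 0's FPCharacterTrace.
; Trace handlers drive its WidgetInteraction component: moves pass a custom hit result, while activate down and up press and release the left mouse button.
; Appear and Dissapear toggle its collision and visibility.
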(event `self.ReceiveBeginPlay`
  (bind _asstart_round_widget (cast `/Game/UI/StartRoundWIdget` (`WidgetComponent.GetUserWidgetObject` (`self.Widget`))))
  (bind _output_get (set `self.MenuWidgetObject` _asstart_round_widget))
  (add `Button.OnClicked` (`/Game/UI/StartRoundWIdget.StartButton` _output_get) (delegate `StartClicked`)))

(event `StartClicked`
  (bind _asfpcharacter_trace (cast `/Game/Blueprints/FPCharacterTrace` (`GameplayStatics.GetPlayerCharacter` 0)))
  (`/Game/Blueprints/FPCharacterTrace.StartWave` _asfpcharacter_trace))

(fn `Appear`
  (`self.SetActorEnableCollision` true)
  (`self.SetActorHiddenInGame` false))

(fn `Dissapear`
  (`self.SetActorEnableCollision` false)
  (`self.SetActorHiddenInGame` true))

(fn `TraceActivateDown`
  (params (hit :type "HitResult Structure (by ref)") (Instigator :type "Pawn Object Reference (by ref)") (TraceType :type "/Game/Blueprints/Interfaces/TypeTraceEnumerator Enum" :default "NewEnumerator0"))
  (returns (Return :type Boolean))
  (`WidgetInteractionComponent.PressPointerKey` (`self.WidgetInteraction`) "LeftMouseButton")
  (return false))

(fn `TraceActivateUp`
  (params (Instigator :type "Pawn Object Reference (by ref)") (hit :type "HitResult Structure (by ref)") (TraceType :type "/Game/Blueprints/Interfaces/TypeTraceEnumerator Enum" :default "NewEnumerator0"))
  (returns (Return :type Boolean))
  (`WidgetInteractionComponent.ReleasePointerKey` (`self.WidgetInteraction`) "LeftMouseButton")
  (return false))

(fn `TraceHitComponet`
  (params (hit :type "HitResult Structure") (component :type "PrimitiveComponent Object Reference") (TraceType :type "/Game/Blueprints/Interfaces/TypeTraceEnumerator Enum" :default "NewEnumerator0"))
  (returns (Return :type Boolean))
  (return false))

(fn `TraceHitObject`
  (params (hit :type "HitResult Structure") (TraceType :type "/Game/Blueprints/Interfaces/TypeTraceEnumerator Enum" :default "NewEnumerator0"))
  (returns (Return :type Boolean))
  (return false))

(fn `TraceLeaveComponent`
  (params (hit :type "HitResult Structure") (component :type "PrimitiveComponent Object Reference") (TraceType :type "/Game/Blueprints/Interfaces/TypeTraceEnumerator Enum" :default "NewEnumerator0"))
  (returns (Return :type Boolean))
  (return false))

(fn `TraceLeaveObject`
  (params (hit :type "HitResult Structure") (TraceType :type "/Game/Blueprints/Interfaces/TypeTraceEnumerator Enum" :default "NewEnumerator0"))
  (returns (Return :type Boolean))
  (return false))

(fn `TraceMove`
  (params (hit :type "HitResult Structure (by ref)") (TraceType :type "/Game/Blueprints/Interfaces/TypeTraceEnumerator Enum" :default "NewEnumerator0"))
  (returns (Return :type Boolean))
  (`WidgetInteractionComponent.SetCustomHitResult` (`self.WidgetInteraction`) hit)
  (return false))

(fn `UserConstructionScript`)