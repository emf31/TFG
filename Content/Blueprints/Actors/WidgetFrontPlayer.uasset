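; WidgetFrontPlayer is an actor that places itself in front of the player character, facing them, shortly after play begins.
; On BeginPlay it waits briefly, then moves to a fixed distance along the character's forward vector and rotates toward the character with a look-at rotation.
; The placement happens once, with no Tick update, so it does not follow later player movement.
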(event `self.ReceiveBeginPlay`
  (bind _returnvalue (`GameplayStatics.GetPlayerCharacter` 0))
  (`KismetSystemLibrary.Delay` 1.0)
  (`self.K2_SetActorLocation` (+ (* (`self.GetActorForwardVector` _returnvalue) 300.0) (`self.K2_GetActorLocation` _returnvalue)))
  (`self.K2_SetActorRotation` (`KismetMathLibrary.FindLookAtRotation` (`self.K2_GetActorLocation`) (`self.K2_GetActorLocation` (`GameplayStatics.GetPlayerCharacter` 0)))))

(fn `UserConstructionScript`)