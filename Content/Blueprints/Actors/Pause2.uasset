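; Pause menu actor that shows a Pause widget in world space, with collision disabled on BeginPlay.
; PutInFrontPlayer places it 200 units ahead of the player character and turns it to face them.
; Trace handlers drive a WidgetInteraction component, feeding hits as custom hit results and activate down/up as left mouse press/release.
; The Continue button is bound on BeginPlay but only prints a debug message.
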(event `self.ReceiveBeginPlay`
  (`self.SetActorEnableCollision` false)
  (bind _aspause (cast `/Game/UI/Pause` (`WidgetComponent.GetUserWidgetObject` (`self.Widget`))))
  (bind _output_get (set `self.PauseWidget` _aspause))
  (add `Button.OnClicked` (`/Game/UI/Pause.Continue` _output_get) (delegate `Whataclick`)))

(event `Whataclick`
  (`KismetSystemLibrary.PrintString` "Le has dado a continue"))

(fn `PutInFrontPlayer`
  (bind _returnvalue (`GameplayStatics.GetPlayerCharacter` 0))
  (`self.K2_SetActorLocation` (+ (* (`self.GetActorForwardVector` _returnvalue) 200.0) (`self.K2_GetActorLocation` _returnvalue)))
  (`self.K2_SetActorRotation` (`KismetMathLibrary.FindLookAtRotation` (`self.K2_GetActorLocation`) (`self.K2_GetActorLocation` (`GameplayStatics.GetPlayerCharacter` 0)))))

(fn `TraceActivateDown`
  (params (hit :type "HitResult Structure (by ref)") (Instigator :type "Pawn Object Reference (by ref)") (TraceType :type "/Game/Blueprints/Interfaces/TypeTraceEnumerator Enum" :default "NewEnumerator0"))
  (returns (Return :type Boolean))
  (`WidgetInteractionComponent.PressPointerKey` (`self.WidgetInteraction`) "LeftMouseButton")
  (return false))

(fn `TraceActivateUp`
  (params (Instigator :type "Pawn Object Reference (by ref)") (hit :type "HitResult Structure (by ref)") (TraceType :type "/Game/Blueprints/Interfaces/TypeTraceEnumerator Enum" :default "NewEnumerator0"))
  (returns (Return :type Boolean))
  (`WidgetInteractionComponent.ReleasePointerKey` (`self.WidgetInteraction`) "LeftMouseButton")
  (return false))

(fn `TraceHitComponet`
  (params (hit :type "HitResult Structure") (component :type "PrimitiveComponent Object Reference") (TraceType :type "/Game/Blueprints/Interfaces/TypeTraceEnumerator Enum" :default "NewEnumerator0"))
  (returns (Return :type Boolean))
  (return false))

(fn `TraceHitObject`
  (params (hit :type "HitResult Structure") (TraceType :type "/Game/Blueprints/Interfaces/TypeTraceEnumerator Enum" :default "NewEnumerator0"))
  (returns (Return :type Boolean))
  (return false))

(fn `TraceLeaveComponent`
  (params (hit :type "HitResult Structure") (component :type "PrimitiveComponent Object Reference") (TraceType :type "/Game/Blueprints/Interfaces/TypeTraceEnumerator Enum" :default "NewEnumerator0"))
  (returns (Return :type Boolean))
  (return false))

(fn `TraceLeaveObject`
  (params (hit :type "HitResult Structure") (TraceType :type "/Game/Blueprints/Interfaces/TypeTraceEnumerator Enum" :default "NewEnumerator0"))
  (returns (Return :type Boolean))
  (return false))

(fn `TraceMove`
  (params (hit :type "HitResult Structure (by ref)") (TraceType :type "/Game/Blueprints/Interfaces/TypeTraceEnumerator Enum" :default "NewEnumerator0"))
  (returns (Return :type Boolean))
  (`WidgetInteractionComponent.SetCustomHitResult` (`self.WidgetInteraction`) hit)
  (return false))

(fn `UserConstructionScript`)