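; Shooting zone trigger actor that plays a Matinee, referenced as a window, when an actor enters and reverses it on exit.
; At BeginPlay it takes the first MatineeActor found in the level as that window sequence.
; Both overlap events also play an audio component from a fixed start offset, with no check on which actor overlaps.
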(event `self.ReceiveBeginPlay`
  (bind _outactors (`GameplayStatics.GetAllActorsOfClass` "/Script/Engine.MatineeActor"))
  (set `self.MatineeWindow` (`KismetArrayLibrary.Array_Get` _outactors)))

(event `self.ReceiveActorBeginOverlap`
  (params (OtherActor :type "Actor Object Reference"))
  (`MatineeActor.Play` (`self.MatineeWindow`))
  (`AudioComponent.Play` (`self.Audio`) 1.71))

(event `self.ReceiveActorEndOverlap`
  (params (OtherActor :type "Actor Object Reference"))
  (`MatineeActor.Reverse` (`self.MatineeWindow`))
  (`AudioComponent.Play` (`self.Audio`) 1.71))

(fn `UserConstructionScript`)