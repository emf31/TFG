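; TeleportVolume is an actor that lets a player teleport to a point they aim at on it.
; Trace interaction callbacks show, move and hide a TeleportVisualizer at the hit, and releasing activate teleports the instigator.
; The destination takes X and Y from the hit and Z from the volume.
; TeleportPlayer offsets it by the pawn-to-camera horizontal difference and BaseEyeHeight, so the camera, not the pawn origin, lands over the target.
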(fn `TeleportPlayer`
  (params (Player :type "Pawn Object Reference") (Location :type "Vector Structure"))
  (bind _asplayer_controller (cast `PlayerController` (`Pawn.GetController` Player)))
  (bind (_returnvalue_x _returnvalue_y) (`KismetMathLibrary.BreakVector` (- (`self.K2_GetActorLocation` Player) (`PlayerCameraManager.GetCameraLocation` (`PlayerController.PlayerCameraManager` _asplayer_controller)))))
  (`self.K2_SetActorLocation` Player (+ (`KismetMathLibrary.MakeVector` _returnvalue_x _returnvalue_y (`Pawn.BaseEyeHeight` Player)) Location) false false))

(fn `TraceActivateDown`
  (params (hit :type "HitResult Structure (by ref)") (Instigator :type "Pawn Object Reference (by ref)"))
  (returns (Return :type Boolean))
  (return false))

(fn `TraceActivateUp`
  (params (Instigator :type "Pawn Object Reference (by ref)") (hit :type "HitResult Structure (by ref)"))
  (returns (Return :type Boolean))
  (bind (_bblockinghit _binitialoverlap _time _location) (`GameplayStatics.BreakHitResult` hit))
  (bind (_returnvalue_x _returnvalue_y _returnvalue_z) (`KismetMathLibrary.BreakVector` (`self.K2_GetActorLocation` self)))
  (`self.TeleportPlayer` Instigator (`KismetMathLibrary.MakeVector` (.x _location) (.y _location) _returnvalue_z))
  (return false))

(fn `TraceHitComponet`
  (params (hit :type "HitResult Structure") (component :type "PrimitiveComponent Object Reference"))
  (returns (Return :type Boolean))
  (return false))

(fn `TraceHitObject`
  (params (hit :type "HitResult Structure"))
  (returns (Return :type Boolean))
  (`SceneComponent.SetVisibility` (`self.TeleportVisualizer`) true true)
  (return false))

(fn `TraceLeaveComponent`
  (params (hit :type "HitResult Structure") (component :type "PrimitiveComponent Object Reference"))
  (returns (Return :type Boolean))
  (return false))

(fn `TraceLeaveObject`
  (params (hit :type "HitResult Structure"))
  (returns (Return :type Boolean))
  (`SceneComponent.SetVisibility` (`self.TeleportVisualizer`) false true)
  (return false))

(fn `TraceMove`
  (params (hit :type "HitResult Structure (by ref)"))
  (returns (Return :type Boolean))
  (`SceneComponent.K2_SetWorldLocation` (`self.TeleportVisualizer`) (`.Location` (`GameplayStatics.BreakHitResult` hit)) false false)
  (return false))

(fn `UserConstructionScript`)