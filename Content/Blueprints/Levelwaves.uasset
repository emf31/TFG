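; Levelwaves runs the zombie wave system, with each wave sized at five zombies times the wave number.
; BeginPlay caches EnemySpawnPoint actors and binds the player character's StartWave and ZombieDead events.
; Starting a wave kicks off GenerateZombieOnWave, which re-arms itself on a random timer, spawning at random points and skipping spawns while paused.
; Deaths are counted until they match the wave total, then WaveEnd is called.
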(event `self.ReceiveBeginPlay`
  ;[1 1 1] Save all zombies spawnPoints
  (bind _outactors (`GameplayStatics.GetAllActorsOfClass` "/Game/Blueprints/EnemySpawnPoint.EnemySpawnPoint_C"))
  (set `self.SpawnPoints` _outactors)
  ;[1 1 1] Bind events that player trigger
  (bind _asfpcharacter_trace (cast `/Game/Blueprints/FPCharacterTrace` (`GameplayStatics.GetPlayerCharacter` 0)))
  (add `/Game/Blueprints/FPCharacterTrace.StartWave` _asfpcharacter_trace (delegate `Start next wave`))
  (add `/Game/Blueprints/FPCharacterTrace.ZombieDead` _asfpcharacter_trace (delegate `ZOmbieDead4WaveSystem`))
  ;[1 1 1] Starting first wave
  (set `self.CurrentWave` 0)
  (`KismetSystemLibrary.Delay` 1.0))

(event `Start next wave`
  ;[1 1 1] Next wave
  (bind _result (`/Engine/EditorBlueprintResources/StandardMacros.IncrementInt` (`self.CurrentWave`))
    (:`  `
      ;[1 1 1] Print number of wave
      (`KismetSystemLibrary.PrintString` (`KismetStringLibrary.Concat_StrStr` "Ronda:" (`KismetStringLibrary.Conv_IntToString` _result)))
      ;[1 1 1] Setting up variables and auxiliar
      (bind _output_get (set `self.NumZombies` (* _result 5)))
      (set `self.ZombiesForAppear` _output_get)
      (set `self.ZombiesDead` 0)
      ;[1 1 1] Generate zombies recursive
      (`KismetSystemLibrary.K2_SetTimer` null "GenerateZombieOnWave" 3.0))))

(event `ZOmbieDead4WaveSystem`
  (bind _zombiesdead (`self.ZombiesDead`))
  ;[1 1 1] If NumZombiesTotales==NumZombies muertos
  (`/Engine/EditorBlueprintResources/StandardMacros.IncrementInt` _zombiesdead
    (:`  `
      (if (== _zombiesdead (`self.NumZombies`))
        ;[1 1 1] Round finished
        (`self.WaveEnd`)))))

(fn `GenerateZombieOnWave`
  (bind _spawnpoints (`self.SpawnPoints`))
  (bind _item (`KismetArrayLibrary.Array_Get` _spawnpoints (`KismetMathLibrary.RandomInteger` (- (`KismetArrayLibrary.Array_Length` _spawnpoints) 1))))
  ;[1 1 1] Generate only if no paused
  (bind _asfpcharacter_trace (cast `/Game/Blueprints/FPCharacterTrace` (`GameplayStatics.GetPlayerCharacter` 0)))
  (if (not (`/Game/Blueprints/FPCharacterTrace.isGamePaused` _asfpcharacter_trace))
    ;[1 1 1] Select one random spawn point and spawn zombie on it
    (`|SpawnActorFromClass` "/Game/Blueprints/AI/ZombieCharacter.ZombieCharacter_C" (`KismetMathLibrary.MakeTransform` (`self.K2_GetActorLocation` _item)) "Undefined" "OverrideRootScale" _item)
    ;[1 1 1] Updating variables wave
    (bind _result (`/Engine/EditorBlueprintResources/StandardMacros.DecrementInt` (`self.ZombiesForAppear`))
      (:`  `
        (if (> _result 0)
          ;[1 1 1] Recursive if not al zombies appeared
          (`KismetSystemLibrary.K2_SetTimer` null "GenerateZombieOnWave" (`KismetMathLibrary.RandomFloatInRange` 1.0 5.0) :!label _label)
          (`KismetSystemLibrary.PrintString` "Aparece zombie")
          (else
            (`KismetSystemLibrary.PrintString` "No quedan zombies por aparecer")))))
    (else
      (goto _label))))

(fn `UserConstructionScript`)