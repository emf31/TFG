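; Test cube that reacts to an interaction trace with color feedback and a surface marker.
; Trace callbacks set the Color material parameter: red when hit, green on activate down, red again on release, white when the trace leaves.
; TraceMove places an Arrow at the hit point, aligned to the surface normal.
; Component-level hit and leave callbacks are stubs, and every callback returns false.
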(fn `TraceActivateDown`
  (params (hit :type "HitResult Structure (by ref)") (Instigator :type "Pawn Object Reference (by ref)"))
  (returns (Return :type Boolean))
  (`KismetSystemLibrary.PrintString` "Hello2")
  (`MeshComponent.SetVectorParameterValueOnMaterials` (`self.Cube`) "Color" (0.0 1.0 0.0))
  (return false))

(fn `TraceActivateUp`
  (params (Instigator :type "Pawn Object Reference (by ref)") (hit :type "HitResult Structure (by ref)"))
  (returns (Return :type Boolean))
  (`MeshComponent.SetVectorParameterValueOnMaterials` (`self.Cube`) "Color" (1.0 0.0 0.0))
  (return false))

(fn `TraceHitComponet`
  (params (hit :type "HitResult Structure") (component :type "PrimitiveComponent Object Reference"))
  (returns (Return :type Boolean))
  (return false))

(fn `TraceHitObject`
  (params (hit :type "HitResult Structure"))
  (returns (Return :type Boolean))
  (`MeshComponent.SetVectorParameterValueOnMaterials` (`self.Cube`) "Color" (1.0 0.0 0.0))
  (return false))

(fn `TraceLeaveComponent`
  (params (hit :type "HitResult Structure") (component :type "PrimitiveComponent Object Reference"))
  (returns (Return :type Boolean))
  (return false))

(fn `TraceLeaveObject`
  (params (hit :type "HitResult Structure"))
  (returns (Return :type Boolean))
  (`MeshComponent.SetVectorParameterValueOnMaterials` (`self.Cube`) "Color" (1.0 1.0 1.0))
  (return false))

(fn `TraceMove`
  (params (hit :type "HitResult Structure (by ref)"))
  (returns (Return :type Boolean))
  (bind (_bblockinghit _binitialoverlap _time _location _impactpoint _normal) (`GameplayStatics.BreakHitResult` hit))
  (`SceneComponent.K2_SetWorldLocationAndRotation` (`self.Arrow`) _location (`KismetMathLibrary.MakeRotFromX` _normal) false false)
  (return false))

(fn `UserConstructionScript`)