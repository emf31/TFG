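; Blueprint interface that lets objects respond to trace-based interaction, such as a pointer or line trace hovering over and activating them.
; It declares hit and leave callbacks at both object and component level, a move callback, and activate down and up calls that carry an instigator.
; Each call receives the hit result and a trace type and returns a value, false in these default stubs.
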(fn `TraceActivateDown`
  (params (hit :type "HitResult Structure (by ref)") (Instigator :type "Pawn Object Reference (by ref)") (TraceType :type "/Game/Blueprints/Interfaces/TypeTraceEnumerator Enum"))
  (returns (Return :type Boolean))
  (return false))

(fn `TraceActivateUp`
  (params (Instigator :type "Pawn Object Reference (by ref)") (hit :type "HitResult Structure (by ref)") (TraceType :type "/Game/Blueprints/Interfaces/TypeTraceEnumerator Enum"))
  (returns (Return :type Boolean))
  (return false))

(fn `TraceHitComponet`
  (params (hit :type "HitResult Structure") (component :type "PrimitiveComponent Object Reference") (TraceType :type "/Game/Blueprints/Interfaces/TypeTraceEnumerator Enum"))
  (returns (Return :type Boolean))
  (return false))

(fn `TraceHitObject`
  (params (hit :type "HitResult Structure") (TraceType :type "/Game/Blueprints/Interfaces/TypeTraceEnumerator Enum"))
  (returns (Return :type Boolean))
  (return false))

(fn `TraceLeaveComponent`
  (params (hit :type "HitResult Structure") (component :type "PrimitiveComponent Object Reference") (TraceType :type "/Game/Blueprints/Interfaces/TypeTraceEnumerator Enum"))
  (returns (Return :type Boolean))
  (return false))

(fn `TraceLeaveObject`
  (params (hit :type "HitResult Structure") (TraceType :type "/Game/Blueprints/Interfaces/TypeTraceEnumerator Enum"))
  (returns (Return :type Boolean))
  (return false))

(fn `TraceMove`
  (params (hit :type "HitResult Structure (by ref)") (TraceType :type "/Game/Blueprints/Interfaces/TypeTraceEnumerator Enum"))
  (returns (Return :type Boolean))
  (return false))