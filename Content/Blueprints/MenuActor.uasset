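; MenuActor is an in-world menu actor whose Start button opens the FPSTraceMap level.
; On BeginPlay it gets the MenuWidget from its Widget component and binds the button's click event.
; Trace callbacks drive a WidgetInteraction component: move feeds it a custom hit result, while activate down and up press and release a virtual left mouse button.
; The other trace callbacks are stubs returning false.
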(event `self.ReceiveBeginPlay`
  (bind _asmenu_widget (cast `/Game/UI/MenuWidget` (`WidgetComponent.GetUserWidgetObject` (`self.Widget`))))
  (bind _output_get (set `self.MenuWidgetObject` _asmenu_widget))
  (add `Button.OnClicked` (`/Game/UI/MenuWidget.StartButton` _output_get) (delegate `StartClicked`)))

(event `StartClicked`
  (`GameplayStatics.OpenLevel` "FPSTraceMap"))

(fn `TraceActivateDown`
  (params (hit :type "HitResult Structure (by ref)") (Instigator :type "Pawn Object Reference (by ref)"))
  (returns (Return :type Boolean))
  (`WidgetInteractionComponent.PressPointerKey` (`self.WidgetInteraction`) "LeftMouseButton")
  (return false))

(fn `TraceActivateUp`
  (params (Instigator :type "Pawn Object Reference (by ref)") (hit :type "HitResult Structure (by ref)"))
  (returns (Return :type Boolean))
  (`WidgetInteractionComponent.ReleasePointerKey` (`self.WidgetInteraction`) "LeftMouseButton")
  (return false))

(fn `TraceHitComponet`
  (params (hit :type "HitResult Structure") (component :type "PrimitiveComponent Object Reference"))
  (returns (Return :type Boolean))
  (return false))

(fn `TraceHitObject`
  (params (hit :type "HitResult Structure"))
  (returns (Return :type Boolean))
  (return false))

(fn `TraceLeaveComponent`
  (params (hit :type "HitResult Structure") (component :type "PrimitiveComponent Object Reference"))
  (returns (Return :type Boolean))
  (return false))

(fn `TraceLeaveObject`
  (params (hit :type "HitResult Structure"))
  (returns (Return :type Boolean))
  (return false))

(fn `TraceMove`
  (params (hit :type "HitResult Structure (by ref)"))
  (returns (Return :type Boolean))
  (`WidgetInteractionComponent.SetCustomHitResult` (`self.WidgetInteraction`) hit)
  (return false))

(fn `UserConstructionScript`)